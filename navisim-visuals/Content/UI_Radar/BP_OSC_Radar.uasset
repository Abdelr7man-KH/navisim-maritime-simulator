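; Radar component that detects boats and surrounding obstacles for its owning actor and streams them over OSC to an external client.
; Two looping half-second timers drive it: a sphere trace sends each "Boat"-tagged actor's name and heading-relative position as a blip.
; A 360-degree line-trace sweep collects hit points in owner-local XY and sends them together as a land message.
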(event Custom|PerformRadarSweep
  (Utilities|Array|Clear (Variables|Default|GetRadarHitPoints))
  (for _index (range 0 (- (Variables|Default|GetSweepResolution) 1))
    (bind (_outhit _returnvalue) (Collision|LineTraceByChannel (Transformation|GetActorLocation (Components|GetOwner)) (+ (* (Math|Vector|RotateVectorAroundAxis (Transformation|GetActorForwardVector (Components|GetOwner)) (Math|Conversions|ToFloat(Integer) (/ (* _index 360) (Variables|Default|GetSweepResolution))) "0.000000,0.000000,1.000000") (Variables|Default|GetRadarRange)) (Transformation|GetActorLocation (Components|GetOwner))) "TraceTypeQuery3" true (Utilities|Array|MakeArray (Components|GetOwner)) "None" true "(R=1.000000,G=0.000000,B=0.000000,A=1.000000)" "(R=0.000000,G=1.000000,B=0.000000,A=1.000000)" 2.0))
    (if _returnvalue
      (Utilities|Array|Add (Variables|Default|GetRadarHitPoints) (Math|Vector2D|MakeVector2D (.x (Math|Transform|InverseTransformLocation (Transformation|GetActorTransform (Components|GetOwner)) (.Location (Collision|BreakHitResult _outhit)))) (.y (Math|Transform|InverseTransformLocation (Transformation|GetActorTransform (Components|GetOwner)) (.Location (Collision|BreakHitResult _outhit))))))))
  (CallFunction|SENDLANDRADAR "/radar/land"))

(event Custom|UpdateEnemyPOS
  (bind _returnvalue (Components|GetOwner))
  (bind _returnvalue_2 (Transformation|GetActorLocation _returnvalue))
  (bind _outhits (Collision|MultiSphereTraceForObjects _returnvalue_2 (+ _returnvalue_2 "0.000000,0.000000,5000.000000") (Variables|Default|GetDetection%20Zone) (Utilities|Array|MakeArray "ObjectTypeQuery3" "ObjectTypeQuery4") false (Utilities|Array|MakeArray _returnvalue) "None" true "(R=1.000000,G=0.000000,B=0.000000,A=1.000000)" "(R=0.000000,G=1.000000,B=0.000000,A=1.000000)" 1.0))
  (for _array_element _outhits
    (if (Actor|ActorHasTag (.HitActor (Collision|BreakHitResult _array_element)) "Boat")
      (CallFunction|SENDRADAR "/radar/blip" (Utilities|GetDisplayName (.HitActor (Collision|BreakHitResult _array_element))) (.X (Math|Vector|BreakVector (Math|Vector|UnrotateVector (- (Transformation|GetActorLocation (.HitActor (Collision|BreakHitResult _array_element))) (Transformation|GetActorLocation (Components|GetOwner))) (Transformation|GetActorRotation (Components|GetOwner))))) (.Y (Math|Vector|BreakVector (Math|Vector|UnrotateVector (- (Transformation|GetActorLocation (.HitActor (Collision|BreakHitResult _array_element))) (Transformation|GetActorLocation (Components|GetOwner))) (Transformation|GetActorRotation (Components|GetOwner)))))))))

(event EventBeginPlay
  (bind _returnvalue (Class|OSCManager|CreateOSCClient "192.168.1.11" 5555 "" 0))
  (Variables|Default|SetOSCSENDRADAR _returnvalue)
  (Utilities|FlowControl|Sequence
    (:then_0
      (Utilities|Time|SetTimerbyEvent (delegate Custom|UpdateEnemyPOS) 0.5 true))
    (:then_1
      (Utilities|Time|SetTimerbyEvent (delegate Custom|PerformRadarSweep) 0.5 true))))

(fn SENDRADAR
  (params (RADARADDRESS :type String) (ShipName :type String%20%28by%20ref%29) (RelativeX :type Float%20%28single-precision%29) (RelativeY :type Float%20%28single-precision%29))
  (bind _returnvalue (Class|OSCManager|ConvertStringtoOSCAddress RADARADDRESS))
  (bind _returnvalue_2 (Class|OSCManager|SetOSCMessageAddress (Utilities|Struct|MakeOSCMessage) _returnvalue))
  (bind _returnvalue_3 (Class|OSCManager|AddString _returnvalue_2 ShipName))
  (bind _returnvalue_4 (Class|OSCManager|AddFloat _returnvalue_3 RelativeX))
  (bind _returnvalue_5 (Class|OSCManager|AddFloat _returnvalue_4 RelativeY))
  (Class|OSCClient|SendOSCMessage (Variables|Default|GetOSCSENDRADAR) _returnvalue_5))

(fn SENDLANDRADAR
  (params (LandAddress :type String))
  (bind _returnvalue (Class|OSCManager|ConvertStringtoOSCAddress LandAddress))
  (bind _returnvalue_2 (Class|OSCManager|SetOSCMessageAddress (Utilities|Struct|MakeOSCMessage) _returnvalue))
  (for _array_element (Variables|Default|GetRadarHitPoints)
    (bind _returnvalue_3 (Class|OSCManager|AddFloat _returnvalue_2 (.x _array_element)))
    (bind _returnvalue_4 (Class|OSCManager|AddFloat _returnvalue_3 (.y _array_element))))
  (Class|OSCClient|SendOSCMessage (Variables|Default|GetOSCSENDRADAR) _returnvalue_4))