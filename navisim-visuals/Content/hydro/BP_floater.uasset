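; BP_floater is an actor that carries a Niagara rain effect, RainForShip, with externally callable rain controls.
; SetRainIntensity writes the given intensity to the effect's User.SpawnRate variable and prints the value to screen.
; ToggleRain is an empty event, as the logic that would activate or deactivate the rain is disconnected and never runs.
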(event Custom|ToggleRain
  (params (TurnOnRain :type Boolean)))

(event Custom|SetRainIntensity
  (params (Intensity :type Float%20%28double-precision%29))
  (Niagara|SetNiagaraVariable(Float) (Variables|Default|GetRainForShip) "User.SpawnRate" Intensity)
  (Development|PrintString (Utilities|String|ToString(Float) Intensity)))

(event EventBeginPlay)

(event Collision|EventActorBeginOverlap
  (params (OtherActor :type Actor%20Object%20Reference)))

(fn ConstructionScript)