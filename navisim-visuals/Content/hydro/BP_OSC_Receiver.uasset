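; OSC bridge between keyboard-driven vessel controls and an external simulation.
; W/S and A/D adjust clamped Nps and Delta, which Tick sends with delta time over OSC and shows on the HUD.
; Incoming messages route by address: state teleports TargetActor in X, Y and yaw, fault zeroes Nps and blocks W, mode toggles pause text.
; Rain handlers are empty stubs, with their BP_floater calls left disconnected.
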(event Custom|OSCMessageRecived
  (params (Message :type OSC%20Message%20Structure%20%28by%20ref%29) (IPAddress :type String) (Port :type Integer))
  (bind _returnvalue (Class|OSCManager|GetOSCMessageAddress Message))
  (bind _returnvalue_2 (Class|OSCManager|GetOSCAddressFullPath _returnvalue))
  (switch string _returnvalue_2
    (:/vessel/state
      (CallFunction|MoveObject))
    (:/instructor/fault
      (CallFunction|IsEngineON))
    (:/system/mode
      (CallFunction|IsPaused123))))

(event Custom|MoveObject
  (bind _targetactor (Variables|Default|GetTargetActor))
  (bind _returnvalue (Transformation|GetActorRotation _targetactor))
  (bind _value (Class|OSCManager|GetFloat (stale Custom|OSCMessageRecived Message)))
  (bind _value_2 (Class|OSCManager|GetFloat (stale Custom|OSCMessageRecived Message) 1))
  (bind _value_3 (Class|OSCManager|GetFloat (stale Custom|OSCMessageRecived Message) 2))
  (Transformation|SetActorLocationAndRotation (Variables|Default|GetTargetActor) (Math|Vector|MakeVector _value _value_2 (.z (Transformation|GetActorLocation (Variables|Default|GetTargetActor)))) (Math|Rotator|MakeRotator (.roll _returnvalue) (.pitch _returnvalue) _value_3) false true))

(event Custom|TurnRainONOFF)

(event Custom|TurnRainOFFFFFFF)

(event Custom|SetRainIntensityOSC)

(event Custom|isEngineON
  (bind _value (Class|OSCManager|GetFloat (stale Custom|OSCMessageRecived Message)))
  (if (== _value 1.0)
    (Variables|Default|SetIsEngineFailed true)
    (Variables|Default|SetCurrentNps 0.0)
    (else
      (Variables|Default|SetIsEngineFailed false))))

(event Custom|isPaused123
  (bind _value (Class|OSCManager|GetFloat (stale Custom|OSCMessageRecived Message)))
  (if (== _value 1.0)
    (Variables|Default|SetIsPaused true)
    (Widget|SetVisibility (Variables|/Game/hydro/WB_SHIPComp.WB_SHIPComp_C|GetPause_Text (Variables|Default|GetMyHUD)) "Visible")
    (else
      (Variables|Default|SetIsPaused false)
      (Widget|SetVisibility (Variables|/Game/hydro/WB_SHIPComp.WB_SHIPComp_C|GetPause_Text (Variables|Default|GetMyHUD)) "Hidden"))))

(event EventBeginPlay
  (Utilities|FlowControl|Sequence
    (:then_0
      (bind _returnvalue (Class|OSCManager|CreateOSCServer "0.0.0.0" 8000 false true "" 0))
      (bind _output_get (Variables|Default|SetOSCServer _returnvalue))
      (EventDispatchers|UnbindallEventsfromOnOscBundleReceived _output_get)
      (EventDispatchers|BindEventtoOnOscMessageReceived _output_get (EventDispatchers|CreateEvent :!event Custom|OSCMessageRecived)))
    (:then_1
      (bind _returnvalue_2 (Class|OSCManager|CreateOSCClient "192.168.1.11" 5555 "" 0))
      (Variables|Default|SetOSCClient _returnvalue_2))
    (:then_2
      (bind _returnvalue_3 (UserInterface|CreateWidget "/Game/hydro/WB_SHIPComp.WB_SHIPComp_C" 0 self))
      (UserInterface|Viewport|AddtoViewport _returnvalue_3 0)
      (bind _output_get_2 (Variables|Default|SetMyHUD _returnvalue_3)))))

(event EventTick
  (params (DeltaSeconds :type Float%20%28single-precision%29))
  (CallFunction|SendOSCMessage "/vessel/input" DeltaSeconds (Variables|Default|GetCurrentNps) (Variables|Default|GetCurrentDelta))
  (Utilities|FlowControl|Sequence
    (:then_0
      (Rendering|Components|TextRender|SetText (Variables|/Game/hydro/WB_SHIPComp.WB_SHIPComp_C|GetNPS_Display (stale EventBeginPlay _output_get_2)) (Utilities|Text|ToText(Float) (Variables|Default|GetCurrentNps) "HalfToEven")))
    (:then_1
      (Rendering|Components|TextRender|SetText (Variables|/Game/hydro/WB_SHIPComp.WB_SHIPComp_C|GetDelta_Display (stale EventBeginPlay _output_get_2)) (Utilities|Text|ToText(Float) (Variables|Default|GetCurrentDelta) "HalfToEven")))))

(event Input|KeyboardEvents|W
  (params (Key :type Key%20Structure :default "None"))
  (:Pressed
    (if (not (Variables|Default|GetIsEngineFailed))
      (Variables|Default|SetCurrentNps (Math|Float|Clamp(Float) (+ (Variables|Default|GetCurrentNps) 1.0) 0.0 15.0)))))

(event Input|KeyboardEvents|S
  (params (Key :type Key%20Structure :default "None"))
  (:Pressed
    (Variables|Default|SetCurrentNps (Math|Float|Clamp(Float) (- (Variables|Default|GetCurrentNps) 1.0) 0.0 15.0))))

(event Input|KeyboardEvents|A
  (params (Key :type Key%20Structure :default "None"))
  (:Pressed
    (Variables|Default|SetCurrentDelta (Math|Float|Clamp(Float) (- (Variables|Default|GetCurrentDelta) 1.0) -35.0 35.0))))

(event Input|KeyboardEvents|D
  (params (Key :type Key%20Structure :default "None"))
  (:Pressed
    (Variables|Default|SetCurrentDelta (Math|Float|Clamp(Float) (+ (Variables|Default|GetCurrentDelta) 1.0) -35.0 35.0))))

(fn ConstructionScript)

(fn SendOSCMessage
  (params (OSCAddress :type String) (dT :type Float%20%28single-precision%29) (nps :type Float%20%28double-precision%29) (delta :type Float%20%28double-precision%29))
  (bind _returnvalue (Class|OSCManager|ConvertStringtoOSCAddress OSCAddress))
  (bind _returnvalue_2 (Class|OSCManager|SetOSCMessageAddress (Utilities|Struct|MakeOSCMessage) _returnvalue))
  (bind _returnvalue_3 (Class|OSCManager|AddFloat _returnvalue_2 dT))
  (bind _returnvalue_4 (Class|OSCManager|AddFloat _returnvalue_3 nps))
  (bind _returnvalue_5 (Class|OSCManager|AddFloat _returnvalue_4 delta))
  (Class|OSCClient|SendOSCMessage (Variables|Default|GetOSCClient) _returnvalue_5))