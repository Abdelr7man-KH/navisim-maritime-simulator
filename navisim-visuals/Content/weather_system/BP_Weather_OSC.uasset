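; Weather controller actor that lets external OSC messages drive storm clouds, lightning, fog, rain and sun position.
; Its OSC server routes each address to a handler that updates a dynamic volumetric cloud material, the fog, the SunSky or rain on BP_Boat_Template.
; Lightning and rain handlers also adjust thunderstorm and rain audio.
; A looping timer runs the day/night clock, updating the sun and orienting the Moon opposite it.
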(event Custom|OSCMessageRecived
  (params (Message :type OSC%20Message%20Structure%20%28by%20ref%29) (IPAddress :type String) (Port :type Integer))
  (bind _returnvalue (Class|OSCManager|GetOSCMessageAddress Message))
  (bind _returnvalue_2 (Class|OSCManager|GetOSCAddressFullPath _returnvalue))
  (switch string _returnvalue_2
    (:/weather/storm/intensity
      (CallFunction|StormIntensity))
    (:/weather/storm/lightning
      (CallFunction|StormLightning))
    (:/weather/fog/density
      (CallFunction|SetFOGDense))
    (:/weather/rain/intensity
      (CallFunction|SetRainIntensityOSC))
    (:/weather/sky/time
      (CallFunction|SetTimeDay))
    (:/weather/sky/rotation
      (CallFunction|SetSunYAW))))

(event Custom|StormLightning
  (bind _value (Class|OSCManager|GetFloat (stale Custom|OSCMessageRecived Message)))
  (Rendering|Material|SetVectorParameterValue (Variables|Default|GetLiveCloudMaterial) "Storm_LightningMasks" (Utilities|Struct|MakeLinearColor _value 5.0 0.5 1.0) :!class /Script/Engine.MaterialInstanceDynamic)
  (if (<= _value 1.0)
    (Audio|Components|Audio|FadeIn (Variables|Default|GetTHUNDERSTORMEFFECT) 2.0 1.0 0.0 "Linear" :!class /Script/Engine.AudioComponent)
    (else
      (Audio|Components|Audio|FadeOut (Variables|Default|GetTHUNDERSTORMEFFECT) 2.0 0.0 "Linear" :!class /Script/Engine.AudioComponent))))

(event Custom|StormIntensity
  (bind _value (Class|OSCManager|GetFloat (stale Custom|OSCMessageRecived Message)))
  (Rendering|Material|SetScalarParameterValue (Variables|Default|GetLiveCloudMaterial) "StormClouds" _value :!class /Script/Engine.MaterialInstanceDynamic)
  (Development|PrintString (Utilities|String|ToString(Float) _value)))

(event Custom|SetFOGDense
  (bind _value (Class|OSCManager|GetFloat (stale Custom|OSCMessageRecived Message)))
  (Class|ExponentialHeightFogComponent|SetFogDensity (Variables|/Script/Engine.ExponentialHeightFog|GetComponent (Variables|Default|GetFogActor)) _value))

(event Custom|SetRainIntensityOSC
  (bind _value (Class|OSCManager|GetFloat (stale Custom|OSCMessageRecived Message)))
  (bind _returnvalue (Actor|GetActorOfClass "/Game/Waterline/7_Vessel_Presets/BP_Boat_Template.BP_Boat_Template_C"))
  (Default|SetRainIntensity _returnvalue _value)
  (Audio|Parameter|SetFloatParameter (Variables|Default|GetAudio_Rain) "RainVolume" (Math|Float|MapRangeClamped _value 0.0 1e+04 0.0 1.0) :!class /Script/Engine.AudioComponent))

(event Custom|SetTimeDay
  (bind _value (Class|OSCManager|GetFloat (stale Custom|OSCMessageRecived Message)))
  (Variables|Default|SetCurrent_Time _value))

(event Custom|SetSunYAW
  (bind _target_sunsky (Variables|Default|GetTarget_SunSky))
  (bind _value (Class|OSCManager|GetFloat (stale Custom|OSCMessageRecived Message)))
  (Variables|/SunPosition/SunSky.SunSky_C|SetNorthOffset _target_sunsky _value)
  (Default|UpdateSun _target_sunsky))

(event Custom|Run_Internal_ClockFORdaynight
  (bind _target_sunsky (Variables|Default|GetTarget_SunSky))
  (bind _output_get (Variables|Default|SetCurrent_Time (Math|Float|%(Float) (+ (Variables|Default|GetCurrent_Time) (Variables|Default|GetTime_Speed)) 24.0)))
  (Variables|/SunPosition/SunSky.SunSky_C|SetSolarTime _target_sunsky _output_get)
  (Default|UpdateSun _target_sunsky)
  (Transformation|SetWorldRotation (Variables|/Script/Engine.Actor|GetRootComponent (Variables|Default|Getmoon)) (Math|Rotator|MakeRotfromX (* (Math|Vector|GetForwardVector (Variables|/SunPosition/SunSky.SunSky_C|GetDirectionalLight _target_sunsky)) "-1.000000,-1.000000,-1.000000")) false false))

(event EventBeginPlay
  (Utilities|FlowControl|Sequence
    (:then_0
      (bind _returnvalue (Class|OSCManager|CreateOSCServer "0.0.0.0" 6767 false true "" 0))
      (bind _output_get (Variables|Default|SetOSCSERver _returnvalue))
      (EventDispatchers|UnbindallEventsfromOnOscBundleReceived _output_get)
      (EventDispatchers|BindEventtoOnOscMessageReceived _output_get (EventDispatchers|CreateEvent :!event Custom|OSCMessageRecived)))
    (:then_1
      (bind _returnvalue_2 (Rendering|Material|CreateDynamicMaterialInstance "/Game/weather_system/storm/MI_stormcloud.MI_stormcloud" "None" "None" :!class /Script/Engine.KismetMaterialLibrary))
      (bind _output_get_2 (Variables|Default|SetLiveCloudMaterial _returnvalue_2))
      (Rendering|Material|SetMaterial (Variables|/SunPosition/SunSky.SunSky_C|GetVolumetricCloud (Variables|Default|GetTarget_SunSky)) _output_get_2))
    (:then_2
      (Utilities|Time|SetTimerbyEvent (delegate Custom|Run_Internal_ClockFORdaynight) 0.1 true))))

(event Collision|EventActorBeginOverlap
  (params (OtherActor :type Actor%20Object%20Reference)))

(event EventTick
  (params (DeltaSeconds :type Float%20%28single-precision%29)))

(fn ConstructionScript)